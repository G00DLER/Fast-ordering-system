(fn CalculateOrderSummary
  (if (and (Variables|Default|GetbAddSugar) (Variables|Default|GetbAddMilk))
    (Variables|Default|SetOrderSummary (Utilities|String|Append "Вы заказали " (Variables|Default|GetSelectedDrink) " C молоком и сахаром"))
    (elif (Variables|Default|GetbAddSugar)
      (Variables|Default|SetOrderSummary (Utilities|String|Append "Вы заказали " (Variables|Default|GetSelectedDrink) " С сахаром"))
      (elif (Variables|Default|GetbAddMilk)
        (Variables|Default|SetOrderSummary (Utilities|String|Append "Вы заказали " (Variables|Default|GetSelectedDrink) " С молоком"))
        (else
          (Variables|Default|SetOrderSummary (Utilities|String|Append "Вы заказали " (Variables|Default|GetSelectedDrink))))))))